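; BP_GM is a game manager Blueprint that advances to the next stage once no actors tagged "Target" remain in the level.
; Its custom event 게임체크 (game check) runs the tag search, then prints a next-stage message and waits briefly when none are found.
; The next level's name comes from the 다음판 (next round) variable on the first BP_StageName actor found, letting that actor define the stage order.
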(event Custom|게임체크
  (bind _outactors (Actor|GetAllActorswithTag "Target"))
  (if (== (Utilities|Array|Length _outactors) 0)
    (Development|PrintString "다음스테이지로")
    (Utilities|FlowControl|Delay 3.0)
    (bind _outactors_2 (Actor|GetAllActorsOfClass "/Game/Blueprint/BP_StageName.BP_StageName_C"))
    (Game|OpenLevel(byName) (Utilities|String|StringToName (Variables|/Game/Blueprint/BP_StageName.BP_StageName_C|Get다음판 (Utilities|Array|Get(acopy) _outactors_2))))))

(fn ConstructionScript)