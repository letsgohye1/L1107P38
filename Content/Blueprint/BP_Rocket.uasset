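; BP_Rocket is a short-lived rocket actor that destroys actors tagged Target on overlap.
; BeginPlay removes the rocket after a brief delay, which caps its lifetime.
; Overlapping a target destroys it, spawns a collapse sound and explosion effect at the rocket, and calls 게임체크 (game check) on the BP_GM game mode before the rocket destroys itself.
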(event Collision|EventActorBeginOverlap
  (params (OtherActor :type Actor%20Object%20Reference))
  (if (Actor|ActorHasTag OtherActor "Target")
    (Actor|DestroyActor OtherActor)
    (Audio|SpawnSoundatLocation "/Game/StarterContent/Audio/Collapse02.Collapse02" (Transformation|GetActorLocation) "0, 0, 0" 1.0 1.0 0.0 0 0)
    (Effects|SpawnEmitteratLocation "/Game/StarterContent/Particles/P_Explosion.P_Explosion" (Transformation|GetActorLocation))
    (bind _asbp_gm (Utilities|Casting|CastToBP_GM (Game|GetGameMode)))
    (Default|게임체크 _asbp_gm)
    (Actor|DestroyActor)))

(event EventBeginPlay
  (Utilities|FlowControl|Delay 0.2)
  (Actor|DestroyActor))

(fn ConstructionScript)